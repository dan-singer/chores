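; Game manager that runs a looping sequence of timed minigames, each with its own instructions, character and duration.
; It shows a task widget, then possesses the minigame's character, readies it and starts a countdown that Tick feeds to the timer widget.
; Timeout shows the lose screen, while OnWin clears the timer and shows the win screen.
; When either screen finishes, it advances to the next minigame, wrapping to the first.
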(event Custom|OnTaskDisplayComplete
  (bind _returnvalue (Game|GetPlayerController 0))
  (bind _minigames (Variables|Default|GetMinigames))
  (bind _currentminigame (Variables|Default|GetCurrentMinigame))
  (bind _output (Utilities|Array|Get(acopy) _minigames _currentminigame))
  (Pawn|UnPossess _returnvalue)
  (Pawn|Possess _returnvalue (.character _output))
  (Class|CharacterBase|MinigameReady (.character _output) (Utilities|Array|Get(acopy) _minigames _currentminigame))
  (Widget|RemovefromParent (Variables|Default|GetTaskWidget))
  (bind _returnvalue_2 (Utilities|Time|SetTimerbyFunctionName 0 "OnTimeout" (.duration _output)))
  (Variables|Default|SetTimerHandle _returnvalue_2)
  (Variables|Default|SetCurTimerDuration (.duration _output))
  (UserInterface|Viewport|AddtoViewport (Variables|Default|GetTimerWidget) 0))

(event Custom|LoseScreenFinished
  (bind _currentminigame (Variables|Default|GetCurrentMinigame))
  (bind _returnvalue (+ _currentminigame 1))
  (Widget|RemovefromParent (Variables|Default|GetLoseWidget))
  (if (>= _returnvalue (Utilities|Array|Length (Variables|Default|GetMinigames)))
    (CallFunction|ActivateMinigame)
    (else
      (CallFunction|ActivateMinigame _returnvalue))))

(event Custom|CustomEvent_0
  (bind _currentminigame (Variables|Default|GetCurrentMinigame))
  (bind _returnvalue (+ _currentminigame 1))
  (Widget|RemovefromParent (Variables|Default|GetWinWidget))
  (if (>= _returnvalue (Utilities|Array|Length (Variables|Default|GetMinigames)))
    (CallFunction|ActivateMinigame)
    (else
      (CallFunction|ActivateMinigame _returnvalue))))

(event EventBeginPlay
  (bind _returnvalue (UserInterface|CreateWidget "/Game/Blueprints/UI/TaskWidget.TaskWidget_C"))
  (bind _output_get (Variables|Default|SetTaskWidget _returnvalue))
  (EventDispatchers|AssignOnTaskDisplayComplete _output_get (delegate Custom|OnTaskDisplayComplete))
  (bind _returnvalue_2 (UserInterface|CreateWidget "/Game/Blueprints/UI/TimerWidget.TimerWidget_C"))
  (Variables|Default|SetTimerWidget _returnvalue_2)
  (bind _returnvalue_3 (UserInterface|CreateWidget "/Game/Blueprints/UI/LoseWidget.LoseWidget_C"))
  (bind _output_get_2 (Variables|Default|SetLoseWidget _returnvalue_3))
  (EventDispatchers|AssignLoseScreenFinished _output_get_2 (delegate Custom|LoseScreenFinished))
  (bind _returnvalue_4 (UserInterface|CreateWidget "/Game/Blueprints/UI/WinWidget.WinWidget_C"))
  (bind _output_get_3 (Variables|Default|SetWinWidget _returnvalue_4))
  (EventDispatchers|AssignWinScreenFinished _output_get_3 (delegate Custom|CustomEvent_0))
  (CallFunction|ActivateMinigame))

(event Collision|EventActorBeginOverlap
  (params (OtherActor :type Actor%20Object%20Reference)))

(event EventTick
  (params (DeltaSeconds :type Float%20%28single-precision%29))
  (if (Utilities|Time|IsValidTimerHandle (Variables|Default|GetTimerHandle))
    (Default|SetProgressPercentage (Variables|Default|GetTimerWidget) (/ (Utilities|Time|GetTimerRemainingTimebyHandle (Variables|Default|GetTimerHandle)) (Variables|Default|GetCurTimerDuration)))))

(fn ConstructionScript)

(fn ActivateMinigame
  (params (GameIndex :type Integer))
  (bind _output_get (Variables|Default|SetCurrentMinigame GameIndex))
  (Default|SetTask (Variables|Default|GetTaskWidget) (.instructions (Utilities|Array|Get(acopy) (Variables|Default|GetMinigames) _output_get)))
  (UserInterface|Viewport|AddtoViewport (Variables|Default|GetTaskWidget) 0))

(fn OnTimeout
  (Widget|RemovefromParent (Variables|Default|GetTimerWidget))
  (UserInterface|Viewport|AddtoViewport (Variables|Default|GetLoseWidget) 0))

(fn OnWin
  (UserInterface|Viewport|AddtoViewport (Variables|Default|GetWinWidget) 0)
  (Widget|RemovefromParent (Variables|Default|GetTimerWidget))
  (Utilities|Time|ClearandInvalidateTimerbyHandle (Variables|Default|GetTimerHandle)))