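; TDDogWalker is the dog walker pawn, likely top-down, that takes over from the first-person walker once the leash is placed.
; Horizontal and Vertical axes drive movement along fixed world axes.
; On LeashPlaced it takes possession, blends the view to Camera, teleports to the first-person walker's location and destroys that actor.
; It then attaches the Dog to itself at a fixed offset.
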(event LeashPlaced(Leash)
  (bind _returnvalue (Game|GetPlayerController 0))
  (bind _fpdogwalker (Variables|Default|GetFPDogWalker))
  (bind _dog (Variables|Default|GetDog))
  (if (Utilities|IsValid _fpdogwalker)
    (Pawn|Possess _returnvalue self)
    (Game|Player|SetViewTargetwithBlend _returnvalue (Variables|Default|GetCamera) 1.0 "VTBlend_Linear" 0.0 false)
    (Transformation|Teleport (Transformation|GetActorLocation _fpdogwalker) "0, 0, 0")
    (Actor|DestroyActor _fpdogwalker)
    (Transformation|AttachActorToActor _dog self "None" "KeepWorld" "KeepRelative" "KeepRelative" true)
    (Transformation|SetActorRelativeLocation _dog "-500.000000, 0, 0")))

(event EventBeginPlay)

(event Collision|EventActorBeginOverlap
  (params (OtherActor :type Actor%20Object%20Reference)))

(event EventTick
  (params (DeltaSeconds :type Float%20%28single-precision%29)))

(event Input|AxisEvents|InputAxisHorizontal
  (params (AxisValue :type Float%20%28single-precision%29))
  (Pawn|Input|AddMovementInput "1.000000, 0, 0" AxisValue false))

(event Input|AxisEvents|InputAxisVertical
  (params (AxisValue :type Float%20%28single-precision%29))
  (Pawn|Input|AddMovementInput "0.000000,-1.000000, 0" AxisValue false))

(fn ConstructionScript)