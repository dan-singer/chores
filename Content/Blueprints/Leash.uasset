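; Leash actor that signals when it has been placed on the dog.
; When its Cube component hits a Dog, it checks that the player character's PhysicsHandleComponent exists and is not grabbing anything.
; It then broadcasts LeashPlaced and sets a BroadcastedEvent flag so the event fires only once.
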(event OnComponentHit(Cube)
  (params (HitComponent :type Primitive%20Component%20Object%20Reference) (OtherActor :type Actor%20Object%20Reference) (OtherComp :type Primitive%20Component%20Object%20Reference) (NormalImpulse :type Vector :default "0, 0, 0") (Hit :type Hit%20Result%20Structure%20%28by%20ref%29))
  (bind _returnvalue (Game|GetPlayerCharacter 0))
  (bind _returnvalue_2 (Actor|GetComponentbyClass _returnvalue "/Script/Engine.PhysicsHandleComponent"))
  (Utilities|Casting|CastToDog OtherActor)
  (if (Utilities|IsValid _returnvalue_2)
    (if (and (not (Utilities|IsValid (Class|PhysicsHandleComponent|GetGrabbedComponent _returnvalue_2))) (Math|Boolean|Equal(Boolean) (Variables|Default|GetbroadcastedEvent) false))
      (Utilities|FlowControl|Sequence
        (:then_0
          (Default|CallLeashPlaced))
        (:then_1
          (Variables|Default|SetbroadcastedEvent true))))))

(event EventBeginPlay)

(event EventTick
  (params (DeltaSeconds :type Float%20%28single-precision%29)))

(fn ConstructionScript)